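; BP_Launchpad is a launchpad actor that throws any Character entering its trigger volume toward a target point.
; On overlap it sets the character's velocity and switches movement to Falling.
; The velocity comes from a custom-arc projectile suggestion, from the character's feet to the local Target converted to world space.
; The construction script sets up a one-way nav link from the pad mesh to Target.
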(event `self.Trigger Volume.OnComponentBeginOverlap`
  (params (OverlappedComponent :type "PrimitiveComponent Object Reference") (OtherActor :type "Actor Object Reference") (OtherComp :type "PrimitiveComponent Object Reference") (OtherBodyIndex :type Integer) (bFromSweep :type Boolean) (SweepResult :type "HitResult Structure (by ref)"))
  (bind _ascharacter (cast `Character` OtherActor))
  (bind _charactermovement (`Character.CharacterMovement` _ascharacter))
  (set `MovementComponent.Velocity` (`self.Calculate Launch Velocity` _ascharacter) _charactermovement)
  (`CharacterMovementComponent.SetMovementMode` _charactermovement "MOVE_Falling" 0))

(fn `Calculate Launch Velocity`
  (params (`Launched Actor` :type "Actor Object Reference"))
  (returns (Velocity :type "Vector Structure"))
  (bind (_origin _boxextent) (`self.GetActorBounds` `Launched Actor` true))
  (bind _outlaunchvelocity (`GameplayStatics.SuggestProjectileVelocity_CustomArc` (- _origin (`KismetMathLibrary.MakeVector` 0.0 0.0 (.z _boxextent))) (`KismetMathLibrary.TransformLocation` (`self.GetTransform`) (`self.Target`))))
  (return _outlaunchvelocity))

(fn `UserConstructionScript`
  (`BlueprintableNavLinkComponent.SetupLink` (`self.BlueprintableNavLink`) (`SceneComponent.RelativeLocation` (`self.Launchpad Mesh`)) (`self.Target`) "LeftToRight"))