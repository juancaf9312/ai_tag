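; BP_TagController is an AI controller that wanders its pawn endlessly between random target points in the level.
; On BeginPlay it caches every TargetPoint as a waypoint, binds to ReceiveMoveCompleted and starts a simple move to a randomly picked one.
; Each completed move, whatever its result, waits briefly and then picks again, so the same waypoint can repeat.
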(event `self.ReceiveBeginPlay`
  (`|ExecutionSequence`
    (:`then_0`
      (bind _outactors (`GameplayStatics.GetAllActorsOfClass` "/Script/Engine.TargetPoint"))
      (set `self.Waypoints` _outactors))
    (:`then_1`
      (add `self.ReceiveMoveCompleted` (delegate `Finished Movement`)))
    (:`then_2`
      (`self.Go To Random Waypoint`))))

(event `Finished Movement` :!signature `self.ReceiveMoveCompleted`
  (params (RequestID :type "AIRequestID Structure") (Result :type "EPathFollowingResult Enum" :default "Success"))
  (`KismetSystemLibrary.Delay` 1.0)
  (`self.Go To Random Waypoint`))

(fn `Get Random Waypoint`
  (returns (Output :type "TargetPoint Object Reference"))
  (bind _waypoints (`self.Waypoints`))
  (return (`|GetArrayItem` _waypoints (`KismetMathLibrary.RandomIntegerInRange` 0 (- (`KismetArrayLibrary.Array_Length` _waypoints) 1)))))

(fn `Go To Random Waypoint`
  (`NavigationSystem.SimpleMoveToActor` self (`self.Get Random Waypoint`)))

(fn `UserConstructionScript`)